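; BP_ThumbnailActor is an editor utility actor that renders a static mesh into a thumbnail texture asset.
; SetUpThumbnailFraming centres the preview mesh by its bounds origin, then places the scene capture diagonally above it, scaled by bounds radius and aimed at the centre.
; It captures to RT_Capture and saves an HDR-compressed static texture through an editor-only call.
; The construction script runs this with an empty name.
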(fn `SetUpThumbnailFraming`
  (params (InStaticMesh :type "StaticMesh Object Reference") (Name :type String))
  (returns (Texture2D :type "Texture2D Object Reference"))
  (bind _previewmeshcomponent (`self.PreviewMeshComponent`))
  (bind _height (`self.Height`))
  (bind _distance (`self.Distance`))
  (bind (_origin _boxextent _sphereradius) (`KismetSystemLibrary.GetComponentBounds` _previewmeshcomponent))
  (bind _returnvalue (* _distance -1.0))
  (`SceneComponent.K2_SetRelativeLocation` (`self.PreviewMeshComponent`) (0.0 0.0 0.0) false false)
  (`StaticMeshComponent.SetStaticMesh` (`self.PreviewMeshComponent`) InStaticMesh)
  (`SceneComponent.K2_SetRelativeLocation` _previewmeshcomponent (* _origin -1.0) false false)
  (`SceneComponent.K2_SetRelativeRotation` :`self` (`self.PreviewMeshComponent`))
  (set `self.Distance` (* _sphereradius 1.0))
  (set `self.Height` (* _sphereradius 1.2))
  (`SceneComponent.K2_SetRelativeLocationAndRotation` (`self.SceneCaptureComponent2D`) (`KismetMathLibrary.MakeVector` _returnvalue _distance _height) (`KismetMathLibrary.FindLookAtRotation` (`KismetMathLibrary.MakeVector` _returnvalue _distance _height) (0.0 0.0 0.0)) false false)
  (`SceneCaptureComponent2D.CaptureScene` (`self.SceneCaptureComponent2D`))
  (bind _returnvalue_2 (`KismetRenderingLibrary.RenderTargetCreateStaticTexture2DEditorOnly` "/Game/Assets/Thumbnails/RT_Capture.RT_Capture" (`local.Name`) "TC_HDR_Compressed"))
  (return _returnvalue_2))

(fn `UserConstructionScript`
  (`self.SetUpThumbnailFraming` (`self.In Static Mesh`)))