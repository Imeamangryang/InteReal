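; Configurable Minotti Jacob coffee table prop whose shape and finishes are picked through selection variables.
; The construction script switches on the model selection to assign one of five meshes: square, circle, small or large rectangle, or triangle.
; It then sets the top, legs and leg detail material slots from three separate material selection variables.
; The event graph holds only disabled stub events, so there is no runtime logic.
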(fn `UserConstructionScript`
  (bind _staticmesh (`self.StaticMesh`))
  (switch `/Game/AS_CoffeeTablesFree/Enums/Enum_SM_CT_Jacob` (`self.ModelSelection`)
    (:`NewEnumerator0`
      (`StaticMeshComponent.SetStaticMesh` _staticmesh "/Game/AS_CoffeeTablesFree/SM/SM_Minotti_Jacob_L_01.SM_Minotti_Jacob_L_01"))
    (:`NewEnumerator1`
      (`StaticMeshComponent.SetStaticMesh` _staticmesh "/Game/AS_CoffeeTablesFree/SM/SM_Minotti_Jacob_Circle_01.SM_Minotti_Jacob_Circle_01"))
    (:`NewEnumerator3`
      (`StaticMeshComponent.SetStaticMesh` _staticmesh "/Game/AS_CoffeeTablesFree/SM/SM_Minotti_Jacob_L_04.SM_Minotti_Jacob_L_04"))
    (:`NewEnumerator4`
      (`StaticMeshComponent.SetStaticMesh` _staticmesh "/Game/AS_CoffeeTablesFree/SM/SM_Minotti_Jacob_L_06.SM_Minotti_Jacob_L_06"))
    (:`NewEnumerator5`
      (`StaticMeshComponent.SetStaticMesh` _staticmesh "/Game/AS_CoffeeTablesFree/SM/SM_Minotti_Jacob_DX_01.SM_Minotti_Jacob_DX_01")))
  (`|ExecutionSequence`
    (:`then_0`
      (`PrimitiveComponent.SetMaterial` (`self.StaticMesh`) 0 (select `/Game/AS_CoffeeTablesFree/Enums/Enum_M_CT_JacobTop` (`self.MaterialSelectionTop`) :`NewEnumerator0` (`self.White Calacatta`) :`NewEnumerator1` (`self.Stone Grey`) :`NewEnumerator2` (`self.Dark Wood`) :`NewEnumerator5` (`self.Brown Wood`) :`NewEnumerator3` (`self.Black Metal`) :`NewEnumerator4` (`self.Color Variation`))))
    (:`then_1`
      (`PrimitiveComponent.SetMaterial` (`self.StaticMesh`) 1 (select `/Game/AS_CoffeeTablesFree/Enums/Enum_M_CT_JacobLegs` (`self.MaterialSelectionLegs`) :`NewEnumerator0` (`self.Dark Wood`) :`NewEnumerator4` (`self.Brown Wood`) :`NewEnumerator1` (`self.Silver`) :`NewEnumerator2` (`self.Bronze`) :`NewEnumerator3` (`self.Black`))))
    (:`then_2`
      (`PrimitiveComponent.SetMaterial` (`self.StaticMesh`) 2 (select `/Game/AS_CoffeeTablesFree/Enums/Enum_M_CT_JacobLegsDetail` (`self.MaterialSelectionLegsDetail`) :`NewEnumerator2` (`self.Bronze`) :`NewEnumerator3` (`self.Black`) :`NewEnumerator1` (`self.Silver`))))))