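; BP_Actor is a harness actor with a PixelStreaming2Peer component and a simple Add function that returns the sum of two values.
; Its BeginPlay and OnStreamerList events are empty.
; Disconnected nodes hold unused player logic that would connect to a local WebSocket, subscribe to the first listed streamer and print a Korean success or failure message.
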(event `self.PixelStreaming2Peer.OnStreamerList`
  (params (StreamerList :type "Array of String (by ref)")))

(event `self.ReceiveBeginPlay`)

(fn `Add`
  (params (Val1 :type Integer) (Val2 :type Integer))
  (returns (Result :type Integer))
  (locals (NewLocalVar :type String))
  (return (+ Val1 Val2)))

(fn `UserConstructionScript`)