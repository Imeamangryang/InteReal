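; Actor that acts as a Pixel Streaming player, receiving a stream inside the game through a PixelStreaming2Peer component.
; On BeginPlay the peer connects to a hardcoded localhost WebSocket address.
; When the streamer list arrives, it subscribes to the first entry and prints a Korean status message, or a failure message if the list is empty.
; A standalone Add helper sums two values and is not called by the event graph.
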(event `self.PixelStreaming2Peer.OnStreamerList`
  (params (StreamerList :type "Array of String (by ref)"))
  (if (> (`KismetArrayLibrary.Array_Length` StreamerList) 0)
    (`PixelStreaming2Peer.Subscribe` (`self.PixelStreaming2Peer`) (`|GetArrayItem` StreamerList))
    (`KismetSystemLibrary.PrintString` "픽셀스트리밍 플레이어 구독중")
    (else
      (`KismetSystemLibrary.PrintString` "픽셀스트리밍 플레이어 연결 실패"))))

(event `self.ReceiveBeginPlay`
  (`PixelStreaming2Peer.Connect` (`self.PixelStreaming2Peer`) "ws://localhost:80"))

(fn `Add`
  (params (Val1 :type Integer) (Val2 :type Integer))
  (returns (Result :type Integer))
  (locals (NewLocalVar :type String))
  (return (+ Val1 Val2)))

(fn `UserConstructionScript`)